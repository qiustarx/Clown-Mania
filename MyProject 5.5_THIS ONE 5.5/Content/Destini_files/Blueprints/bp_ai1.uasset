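; AI character Blueprint that chases the player on sight and plays an attack montage on reaching them.
; PawnSensing sets a seen flag and calls FollowPlayer, which runs AI MoveTo toward the player and, on success, plays the montage behind a CanAttack gate timed to its length.
; Tick halts movement while the flag is false, but nothing clears the flag once it is set.
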(event OnSeePawn(PawnSensing)
  (params (Pawn :type Pawn%20Object%20Reference))
  (Variables|Default|SetIsSeeingPlayer? true)
  (CallFunction|FollowPlayer))

(event Custom|FollowPlayer
  (Variables|Default|SetCanAttack? true)
  (if (Variables|Default|GetIsSeeingPlayer?)
    (AI|AIMoveTo self "0, 0, 0" (Game|GetPlayerCharacter 0) 7e+01 false
      (:OnSuccess
        (if (Variables|Default|GetCanAttack?)
          (Variables|Default|SetCanAttack? false)
          (bind _returnvalue (Animation|PlayAnimMontage 0 1.0 "None"))
          (Utilities|FlowControl|Delay _returnvalue)
          (Variables|Default|SetCanAttack? true))))
    (else
      (Variables|Default|SetIsSeeingPlayer? false))))

(event EventTick
  (params (DeltaSeconds :type Float%20%28single-precision%29))
  (if (not (Variables|Default|GetIsSeeingPlayer?))
    (Components|Movement|StopMovementImmediately (Variables|Character|GetCharacterMovement))))

(fn ConstructionScript)