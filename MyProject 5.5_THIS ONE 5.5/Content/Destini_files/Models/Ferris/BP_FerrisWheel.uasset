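; Ferris wheel actor that starts spinning on BeginPlay and responds to two trigger volumes.
; A rotation timeline turns the wheel mesh, while start, stop and slow timelines ramp its play rate.
; Overlapping the controls trigger toggles the wheel on or off; the entrance trigger slows it and replays the start ramp on exit.
; Each update resets the ten carts' world rotation from the actor's pitch and yaw to keep them level.
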(event OnComponentBeginOverlap(Trigger_Controls)
  (params (OverlappedComponent :type Primitive%20Component%20Object%20Reference) (OtherActor :type Actor%20Object%20Reference) (OtherComp :type Primitive%20Component%20Object%20Reference) (OtherBodyIndex :type Integer) (bFromSweep :type Boolean) (SweepResult :type Hit%20Result%20Structure%20%28by%20ref%29))
  (if (Variables|Setup|GetActive)
    (CallFunction|EventStopWheel)
    (Variables|Setup|SetActive false)
    (else
      (CallFunction|EventStartWheel)
      (Variables|Setup|SetActive true))))

(event OnComponentEndOverlap(Trigger_Entrance)
  (params (OverlappedComponent :type Primitive%20Component%20Object%20Reference) (OtherActor :type Actor%20Object%20Reference) (OtherComp :type Primitive%20Component%20Object%20Reference) (OtherBodyIndex :type Integer))
  (CallFunction|EventStartWheel))

(event OnComponentBeginOverlap(Trigger_Entrance)
  (params (OverlappedComponent :type Primitive%20Component%20Object%20Reference) (OtherActor :type Actor%20Object%20Reference) (OtherComp :type Primitive%20Component%20Object%20Reference) (OtherBodyIndex :type Integer) (bFromSweep :type Boolean) (SweepResult :type Hit%20Result%20Structure%20%28by%20ref%29))
  (bind _alpha (Timeline|TM_Wheel_Slow PlayFromStart)
    (:Update
      (Variables|Setup|SetCurrentRate (Math|Float|Lerp (Variables|Setup|GetRotationRate) (Variables|Setup|GetEntranceRate) _alpha))
      (Components|Timeline|SetPlayRate (Variables|Default|GetTM_Wheel_Rotation) (Variables|Setup|GetCurrentRate)))))

(event Custom|EventRotateWheel
  (Components|Timeline|SetPlayRate (Variables|Default|GetTM_Wheel_Rotation) (Variables|Setup|GetCurrentRate))
  (bind _alpha (Timeline|TM_Wheel_Rotation Play)
    (:Update
      (Transformation|SetRelativeRotation (Variables|Default|GetFW_Wheel) (Math|Rotator|Lerp(Rotator) "0, 0, 0" "0, 0,359.000000" _alpha) false false)
      (|ROTATECARTS))))

(event Custom|EventStopWheel
  (bind _alpha (Timeline|TM_Wheel_Stop PlayFromStart)
    (:Update
      (Variables|Setup|SetCurrentRate (Math|Float|Lerp (Variables|Setup|GetRotationRate) 0.0 _alpha))
      (Components|Timeline|SetPlayRate (Variables|Default|GetTM_Wheel_Rotation) (Variables|Setup|GetCurrentRate)))))

(event Custom|EventStartWheel
  (bind _alpha (Timeline|TM_Wheel_Start PlayFromStart)
    (:Update
      (Variables|Setup|SetCurrentRate (Math|Float|Lerp 0.0 (Variables|Setup|GetRotationRate) _alpha))
      (Components|Timeline|SetPlayRate (Variables|Default|GetTM_Wheel_Rotation) (Variables|Setup|GetCurrentRate)))))

(event EventBeginPlay
  (CallFunction|EventStartWheel)
  (CallFunction|EventRotateWheel))

(fn ConstructionScript)